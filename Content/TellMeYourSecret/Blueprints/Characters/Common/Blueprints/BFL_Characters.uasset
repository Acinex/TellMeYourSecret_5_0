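; Blueprint function library that computes smoothed head and eye look-at rotations for characters aiming at a target point.
; The raw rotation runs from a mesh socket to the target, with pitch inverted, yaw relative to the actor, and axes wrapped toward ±180 degrees.
; The head interpolates toward that rotation within its pitch and yaw limits.
; The eyes interpolate toward the remainder left by the smoothed head, using their own limits and speed.
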(fn CalculateLookatRotations
  (params (Character :type Character%20Object%20Reference) (CharacterMesh :type Skeletal%20Mesh%20Component%20Object%20Reference) (SourceBone :type Name) (LookAtTarget :type Vector) (HeadRotationConstraint :type STR%20Rotation%20Constraint%20Structure) (EyeRotationConstraint :type STR%20Rotation%20Constraint%20Structure) (InHeadLookAtRotation :type Rotator) (InEyeLookAtRotation :type Rotator))
  (bind (_minroll _maxroll _minpitch _maxpitch _minyaw _maxyaw _speed) (Utilities|Struct|BreakSTR_RotationConstraint HeadRotationConstraint))
  (bind (_minroll_2 _maxroll_2 _minpitch_2 _maxpitch_2 _minyaw_2 _maxyaw_2 _speed_2) (Utilities|Struct|BreakSTR_RotationConstraint EyeRotationConstraint))
  (bind _returnvalue (Transformation|GetSocketLocation CharacterMesh SourceBone))
  (bind _returnvalue_2 (Math|Rotator|FindLookatRotation _returnvalue LookAtTarget))
  (bind (_roll _pitch _yaw) (Math|Rotator|BreakRotator _returnvalue_2))
  ;[1 1 1] Calculate raw look at rotation
  (bind _out_rotator (CallFunction|RemapLookatRotator (Math|Rotator|MakeRotator _roll (* _pitch -1.0) (- _yaw (.Yaw (Math|Rotator|BreakRotator (Transformation|GetActorRotation Character)))))))
  (bind _output_get (LocalVariables|SetRawLookAtRotation _out_rotator))
  (return (Math|Interpolation|RInterpTo InHeadLookAtRotation (Math|Rotator|MakeRotator (.Roll (Math|Rotator|BreakRotator _output_get)) (Math|Float|Clamp(Float) (.Pitch (Math|Rotator|BreakRotator _output_get)) _minpitch _maxpitch) (Math|Float|Clamp(Float) (.Yaw (Math|Rotator|BreakRotator _output_get)) _minyaw _maxyaw)) (Utilities|Time|GetWorldDeltaSeconds) _speed) (Math|Interpolation|RInterpTo InEyeLookAtRotation (Math|Rotator|MakeRotator (.Roll (Math|Rotator|BreakRotator (Math|Rotator|MakeRotator (.Roll (Math|Rotator|BreakRotator (LocalVariables|GetRawLookAtRotation))) (- (.Pitch (Math|Rotator|BreakRotator (LocalVariables|GetRawLookAtRotation))) (.Pitch (Math|Rotator|BreakRotator (Math|Interpolation|RInterpTo InHeadLookAtRotation (Math|Rotator|MakeRotator (.Roll (Math|Rotator|BreakRotator _output_get)) (Math|Float|Clamp(Float) (.Pitch (Math|Rotator|BreakRotator _output_get)) _minpitch _maxpitch) (Math|Float|Clamp(Float) (.Yaw (Math|Rotator|BreakRotator _output_get)) _minyaw _maxyaw)) (Utilities|Time|GetWorldDeltaSeconds) _speed)))) (- (.Yaw (Math|Rotator|BreakRotator (LocalVariables|GetRawLookAtRotation))) (.Yaw (Math|Rotator|BreakRotator (Math|Interpolation|RInterpTo InHeadLookAtRotation (Math|Rotator|MakeRotator (.Roll (Math|Rotator|BreakRotator _output_get)) (Math|Float|Clamp(Float) (.Pitch (Math|Rotator|BreakRotator _output_get)) _minpitch _maxpitch) (Math|Float|Clamp(Float) (.Yaw (Math|Rotator|BreakRotator _output_get)) _minyaw _maxyaw)) (Utilities|Time|GetWorldDeltaSeconds) _speed))))))) (Math|Float|Clamp(Float) (.Pitch (Math|Rotator|BreakRotator (Math|Rotator|MakeRotator (.Roll (Math|Rotator|BreakRotator (LocalVariables|GetRawLookAtRotation))) (- (.Pitch (Math|Rotator|BreakRotator (LocalVariables|GetRawLookAtRotation))) (.Pitch (Math|Rotator|BreakRotator (Math|Interpolation|RInterpTo InHeadLookAtRotation (Math|Rotator|MakeRotator (.Roll (Math|Rotator|BreakRotator _output_get)) (Math|Float|Clamp(Float) (.Pitch (Math|Rotator|BreakRotator _output_get)) _minpitch _maxpitch) (Math|Float|Clamp(Float) (.Yaw (Math|Rotator|BreakRotator _output_get)) _minyaw _maxyaw)) (Utilities|Time|GetWorldDeltaSeconds) _speed)))) (- (.Yaw (Math|Rotator|BreakRotator (LocalVariables|GetRawLookAtRotation))) (.Yaw (Math|Rotator|BreakRotator (Math|Interpolation|RInterpTo InHeadLookAtRotation (Math|Rotator|MakeRotator (.Roll (Math|Rotator|BreakRotator _output_get)) (Math|Float|Clamp(Float) (.Pitch (Math|Rotator|BreakRotator _output_get)) _minpitch _maxpitch) (Math|Float|Clamp(Float) (.Yaw (Math|Rotator|BreakRotator _output_get)) _minyaw _maxyaw)) (Utilities|Time|GetWorldDeltaSeconds) _speed))))))) _minpitch_2 _maxpitch_2) (Math|Float|Clamp(Float) (.Yaw (Math|Rotator|BreakRotator (Math|Rotator|MakeRotator (.Roll (Math|Rotator|BreakRotator (LocalVariables|GetRawLookAtRotation))) (- (.Pitch (Math|Rotator|BreakRotator (LocalVariables|GetRawLookAtRotation))) (.Pitch (Math|Rotator|BreakRotator (Math|Interpolation|RInterpTo InHeadLookAtRotation (Math|Rotator|MakeRotator (.Roll (Math|Rotator|BreakRotator _output_get)) (Math|Float|Clamp(Float) (.Pitch (Math|Rotator|BreakRotator _output_get)) _minpitch _maxpitch) (Math|Float|Clamp(Float) (.Yaw (Math|Rotator|BreakRotator _output_get)) _minyaw _maxyaw)) (Utilities|Time|GetWorldDeltaSeconds) _speed)))) (- (.Yaw (Math|Rotator|BreakRotator (LocalVariables|GetRawLookAtRotation))) (.Yaw (Math|Rotator|BreakRotator (Math|Interpolation|RInterpTo InHeadLookAtRotation (Math|Rotator|MakeRotator (.Roll (Math|Rotator|BreakRotator _output_get)) (Math|Float|Clamp(Float) (.Pitch (Math|Rotator|BreakRotator _output_get)) _minpitch _maxpitch) (Math|Float|Clamp(Float) (.Yaw (Math|Rotator|BreakRotator _output_get)) _minyaw _maxyaw)) (Utilities|Time|GetWorldDeltaSeconds) _speed))))))) _minyaw_2 _maxyaw_2)) (Utilities|Time|GetWorldDeltaSeconds) _speed_2)))

(fn RemapLookatRotator
  (params (In%20Rotator :type Rotator))
  (bind (_roll _pitch _yaw) (Math|Rotator|BreakRotator In%20Rotator))
  (return (Math|Rotator|MakeRotator (CallFunction|MapAxis _roll) (CallFunction|MapAxis _pitch) (CallFunction|MapAxis _yaw))))

(fn MapAxis
  (params (In%20Value :type Float%20%28single-precision%29))
  (bind _returnvalue (- In%20Value 3.6e+02))
  (bind _returnvalue_2 (> In%20Value 1.8e+02))
  (bind _returnvalue_3 (Math|Float|SelectFloat _returnvalue In%20Value _returnvalue_2))
  (return (Math|Float|SelectFloat (+ _returnvalue_3 3.6e+02) _returnvalue_3 (< _returnvalue_3 -1.8e+02))))