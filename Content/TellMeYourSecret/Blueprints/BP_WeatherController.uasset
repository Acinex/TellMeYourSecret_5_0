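; BP_WeatherController is a weather actor that runs one timed rain shower shortly after BeginPlay.
; StartRain and EndRain toggle the Rain component and flip the sign of ChangeRate.
; Each tick, SetRainLevel adds that rate to the "Rain" scalar in the MP_Global parameter collection while it differs from RainLevel.
; UpdateSky is also called each tick, but its cloud opacity logic is disconnected, so it does nothing.
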(event Custom|Start%20Rain
  (Components|Activation|SetActive (Variables|Default|GetRain) true false)
  (Variables|Default|SetChangeRate 0.001))

(event Custom|End%20Rain
  (Components|Activation|SetActive (Variables|Default|GetRain) false false)
  (Variables|Default|SetChangeRate -0.001))

(event EventBeginPlay
  (Utilities|FlowControl|Delay 5.0)
  (CallFunction|StartRain)
  (Utilities|FlowControl|Delay 3e+01)
  (CallFunction|EndRain))

(event Collision|EventActorBeginOverlap
  (params (OtherActor :type Actor%20Object%20Reference)))

(event EventTick
  (params (DeltaSeconds :type Float%20%28single-precision%29))
  (|UpdateSky)
  (|SetRainLevel))

(fn ConstructionScript)